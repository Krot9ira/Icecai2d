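; Base breakable actor that takes damage and is destroyed when its health runs out.
; AnyDamage subtracts the truncated damage from a Health component and calls SpawnDestructible once health reaches zero or below.
; SpawnDestructible uses a DoOnce to spawn the DestroyEffect particle system at the static mesh's transform a single time, then destroys the actor.
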(event `self.ReceiveAnyDamage`
  (params (Damage :type "Float (single-precision)") (DamageType :type "DamageType Object Reference") (InstigatedBy :type "Controller Object Reference") (DamageCauser :type "Actor Object Reference"))
  (bind _health (`self.Health`))
  (`HealthComponent.RemoveHealth` _health (`KismetMathLibrary.FTrunc` Damage))
  (bind _returnvalue (`HealthComponent.GetHealth` _health))
  (if (<= _returnvalue 0)
    (`self.SpawnDestructible` null)))

(event `SpawnDestructible`
  (params (DestroyedActor :type "Actor Object Reference"))
  (`/Engine/EditorBlueprintResources/StandardMacros.DoOnce` false
    (:`Completed`
      (`NiagaraFunctionLibrary.SpawnSystemAtLocation` (`self.DestroyEffect`) (.location (`SceneComponent.K2_GetComponentToWorld` (`self.StaticMesh`))) (.rotation (`SceneComponent.K2_GetComponentToWorld` (`self.StaticMesh`))) (.scale (`SceneComponent.K2_GetComponentToWorld` (`self.StaticMesh`))))
      (`self.K2_DestroyActor`))))

(fn `UserConstructionScript`)