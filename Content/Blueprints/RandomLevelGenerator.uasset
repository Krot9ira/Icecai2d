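; Random level generator actor that builds an AxisX by AxisY grid of streamed level tiles on BeginPlay.
; Each cell takes a random level from LevelNames, or from its SpecificLevelInfo entry when the 1-based coordinates match.
; GenerateLevel creates a uniquely named streaming-level instance per cell, then loads and shows it.
; Tiles are spaced by LevelSize around the world origin, with a quarter-tile Y skew and random 90-degree yaw steps.
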(event `self.ReceiveBeginPlay`
  (bind _axisy (`self.AxisY`))
  (bind _axisx (`self.AxisX`))
  (bind _loopx (`self.LoopX`))
  (bind _loopy (`self.LoopY`))
  (`KismetSystemLibrary.PrintString` "Hello")
  (for _index (range (`self.AxisX`))
    (set `self.LoopX` _index)
    (for _index_2 (range (`self.AxisY`))
      (set `self.LoopY` _index_2)
      (bind (_returnvalue _array_element) (`self.CheckForSpecificAxis` (`self.SpecificLevelInfo`) (`self.LoopX`) (`self.LoopY`)))
      (if _returnvalue
        (`self.GenerateLevel` (`.LevelNames_6_1C91E0E54BB8F0E471110AB3271ACC18` (break `/Game/Data/Structure/SpecificLevelInfo` _array_element)) _loopx _loopy _axisx _axisy)
        (else
          (`self.GenerateLevel` (`self.LevelNames`) _loopx _loopy _axisx _axisy))))))

(event `self.ReceiveTick`
  (params (DeltaSeconds :type "Float (single-precision)")))

(fn `CheckForSpecificAxis`
  (params (Array :type "Array of /Game/Data/Structure/SpecificLevelInfo Structure") (B :type Integer) (B1 :type Integer))
  (returns (ReturnValue :type Boolean) (`Array Element` :type "/Game/Data/Structure/SpecificLevelInfo Structure"))
  (for _array_element Array
    (bind _returnvalue (and (== (- (`KismetMathLibrary.Round` (.x (`.Coordinates_2_8A67BD8045562ED612994BB4A0B56989` (break `/Game/Data/Structure/SpecificLevelInfo` _array_element)))) 1) B) (== (- (`KismetMathLibrary.Round` (.y (`.Coordinates_2_8A67BD8045562ED612994BB4A0B56989` (break `/Game/Data/Structure/SpecificLevelInfo` _array_element)))) 1) B1)))
    (if _returnvalue
      (return _returnvalue _array_element)))
  (return false))

(fn `GenerateLevel`
  (params (Array :type "Array of Name") (LoopX :type Integer) (LoopY :type Integer) (X :type Integer) (Y :type Integer))
  (`KismetSystemLibrary.PrintString` "genete" true true (struct :`R` 1.0 :`B` 0.600873 :`A` 1.0) 22.0)
  (bind _returnvalue (`LevelStreaming.CreateInstance` (`GameplayStatics.GetStreamingLevel` (`|GetArrayItem` Array (`KismetMathLibrary.RandomIntegerInRange` 0 (`KismetArrayLibrary.Array_LastIndex` Array)))) (`KismetStringLibrary.Concat_StrStr` (`KismetStringLibrary.Conv_IntToString` LoopX) "x" (`KismetStringLibrary.Conv_IntToString` LoopY))))
  (set `LevelStreaming.LevelTransform` (`KismetMathLibrary.MakeTransform` (`KismetMathLibrary.MakeVector` (+ (- (* LoopX (`self.LevelSize`)) (/ (* X (`self.LevelSize`)) 2.0)) (/ (`self.LevelSize`) 2.0)) (+ (- (* LoopY (`self.LevelSize`)) (/ (* Y (`self.LevelSize`)) 2.0)) (/ (/ (`self.LevelSize`) 2.0) 2.0))) (`KismetMathLibrary.MakeRotator` 0.0 0.0 (`KismetMathLibrary.Conv_IntToDouble` (* (`KismetMathLibrary.RandomIntegerInRange` 0 3) 90)))) _returnvalue)
  (set `LevelStreaming.bShouldBeLoaded` true _returnvalue)
  (set `LevelStreaming.bShouldBeVisible` true _returnvalue))

(fn `UserConstructionScript`)