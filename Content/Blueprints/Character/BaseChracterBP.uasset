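; Base character Blueprint that equips a melee weapon and provides a procedural walk animation.
; On BeginPlay it spawns a BaseMeleBP with itself as instigator, stores it in WeaponRef and snaps it to the Spline component.
; AnimWalk plays a timeline that moves the mesh's relative location along Spline1, swapping the X and Z axes.
; Tick does nothing, and a delayed weapon attack call is left unconnected.
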(event `self.ReceiveBeginPlay`
  (`self.SpawnWeapon`)
  (`/Engine/EditorBlueprintResources/StandardMacros.IsValid` (`self.GetInstigator`)))

(event `SpawnWeapon`
  (bind _spline (`self.Spline`))
  (bind _returnvalue (`|SpawnActorFromClass` "/Game/Blueprints/Weapon/Mele/BaseMeleBP.BaseMeleBP_C" (`SceneComponent.K2_GetComponentToWorld` _spline) "Undefined" "OverrideRootScale" null self))
  (bind _output_get (set `self.WeaponRef` _returnvalue))
  (`self.K2_AttachToComponent` _output_get _spline "None" "SnapToTarget" "SnapToTarget" "SnapToTarget" true))

(event `AnimWalk`
  (bind (_direction _tack) (`Timeline|TimeLineWalk` :!via `PlayFromStart`)
    (:`Update`
      (`SceneComponent.K2_SetRelativeLocation` (`self.Mesh`) (`KismetMathLibrary.MakeVector` (.z (.location (`SplineComponent.GetTransformAtTime` (`self.Spline1`) _tack "Local" false false))) (.y (.location (`SplineComponent.GetTransformAtTime` (`self.Spline1`) _tack "Local" false false))) (.x (.location (`SplineComponent.GetTransformAtTime` (`self.Spline1`) _tack "Local" false false)))) false false))))

(event `self.ReceiveTick`
  (params (DeltaSeconds :type "Float (single-precision)"))
  (set `self.Delta Seconds` DeltaSeconds))

(fn `UserConstructionScript`)