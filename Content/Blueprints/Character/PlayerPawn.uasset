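; Player pawn for click-to-move control that spawns an AI-driven character and follows its capsule location every tick.
; While LMB is held, a looping timer traces under the cursor and writes the character's NavPoint blackboard key.
; The target is the hit interactable or character, otherwise a reusable navigation marker actor placed at the hit location.
; An X-bounds camera check is stubbed: nothing here calls it and MoveCameraX is empty.
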(event `self.ReceiveBeginPlay`
  (bind _returnvalue (`|SpawnActorFromClass` "/Game/Blueprints/Character/BaseChracterBP.BaseChracterBP_C" (`SceneComponent.K2_GetComponentToWorld` (`self.DefaultSceneRoot`)) "Undefined" "OverrideRootScale" null self))
  (set `self.ControlledChracter` _returnvalue)
  (set `PlayerController.bShowMouseCursor` true (`GameplayStatics.GetPlayerController` 0))
  (`self.K2_SetActorRelativeLocation` (-50.0 0.0 100.0))
  (`KismetSystemLibrary.ExecuteConsoleCommand` "stat fps" null))

(event `InputAction|LMB`
  (params (Key :type "Key Structure"))
  (:`Pressed`
    (bind _returnvalue (`KismetSystemLibrary.K2_SetTimerDelegate` (delegate `SetMoveObject`) 0.05 true))
    (set `self.LMBPressedTimer` _returnvalue))
  (:`Released`
    (`KismetSystemLibrary.K2_ClearAndInvalidateTimerHandle` (`self.LMBPressedTimer`))))

(event `SetMoveObject`
  (bind _navpoint (`self.NavPoint`))
  (bind _returnvalue (`AIBlueprintHelperLibrary.GetBlackboard` (`self.ControlledChracter`)))
  (bind (_bblockinghit _binitialoverlap _time _distance _location _impactpoint _normal _impactnormal _physmat _hitactor) (`GameplayStatics.BreakHitResult` (`PlayerController.GetHitResultUnderCursorByChannel` (`GameplayStatics.GetPlayerController` 0) "TraceTypeQuery1" false)))
  (bind _asbase_interactble (cast `/Game/Blueprints/Enviroment/BaseInteractble` _hitactor)
    (:`then`
      (`BlackboardComponent.SetValueAsObject` (`AIBlueprintHelperLibrary.GetBlackboard` (`self.ControlledChracter`)) (`self.NavPoint`) _asbase_interactble))
    (:`CastFailed`
      (bind _asbase_character (cast `BaseCharacter` _hitactor)
        (:`then`
          (`BlackboardComponent.SetValueAsObject` _returnvalue _navpoint _asbase_character))
        (:`CastFailed`
          (`/Engine/EditorBlueprintResources/StandardMacros.IsValid` (`self.NavigationPointRef`)
            (:`Is Valid`
              (`self.K2_SetActorLocation` (`self.NavigationPointRef`) _location false false))
            (:`Is Not Valid`
              (bind _returnvalue_2 (`|SpawnActorFromClass` "/Game/Blueprints/Character/NavigationPointBP.NavigationPointBP_C" (`KismetMathLibrary.MakeTransform` _location) "Undefined" "OverrideRootScale" null null))
              (set `self.NavigationPointRef` _returnvalue_2)))
          (`BlackboardComponent.SetValueAsObject` _returnvalue _navpoint (`self.NavigationPointRef`)))))))

(event `self.ReceiveTick`
  (params (DeltaSeconds :type "Float (single-precision)"))
  (`self.K2_SetActorLocation` (`SceneComponent.K2_GetComponentLocation` (`Character.CapsuleComponent` (`self.ControlledChracter`)))))

(event `CheckPlayerX`
  (bind _x (.x (`self.K2_GetActorLocation` (`self.ControlledChracter`))))
  (if (and (< (+ (`self.MaxX`) (`self.MapCenter`)) _x) (> _x (+ (`self.MapCenter`) (`self.MinX`))))
    (`self.MoveCameraX`)))

(event `MoveCameraX`)

(fn `UserConstructionScript`)