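; Player pawn for point-and-click control of a separately spawned, AI-driven character.
; On BeginPlay it spawns and stores a BaseChracterBP, shows the mouse cursor and offsets its own location.
; Left click spawns a NavigationPointBP at the cursor hit and writes it to the character's blackboard as NavPoint.
; An unconnected node would attach the pawn to the character but never runs.
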(event `self.ReceiveBeginPlay`
  (bind _returnvalue (`|SpawnActorFromClass` "/Game/Blueprints/Character/BaseChracterBP.BaseChracterBP_C" (`SceneComponent.K2_GetComponentToWorld` (`self.CollisionComponent`)) "Undefined" "OverrideRootScale" null self))
  (set `self.ControlledChracter` _returnvalue)
  (set `PlayerController.bShowMouseCursor` true (`GameplayStatics.GetPlayerController` 0))
  (`self.K2_SetActorRelativeLocation` (-50.0 0.0 100.0)))

(event `Key|LeftMouseButton`
  (params (Key :type "Key Structure"))
  (:`Pressed`
    (bind _returnvalue (`|SpawnActorFromClass` "/Game/Blueprints/Character/NavigationPointBP.NavigationPointBP_C" (`KismetMathLibrary.MakeTransform` (`.Location` (`GameplayStatics.BreakHitResult` (`PlayerController.GetHitResultUnderCursorByChannel` (`GameplayStatics.GetPlayerController` 0) "TraceTypeQuery1" false)))) "Undefined" "OverrideRootScale" null null))
    (`BlackboardComponent.SetValueAsObject` (`AIBlueprintHelperLibrary.GetBlackboard` (`self.ControlledChracter`)) (`self.NavPoint`) _returnvalue)))

(fn `UserConstructionScript`)