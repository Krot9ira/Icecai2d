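; Base melee weapon actor that animates a swing along a spline on its instigating BaseChracterBP and attacks what its mesh overlaps.
; AnimateAttack triggers a DoOnce-gated swing that toggles mesh visibility and starts a looping timer.
; Each timer step enables overlap events and advances the weapon along the spline using AttackSpeed and Tick's cached delta.
; At the spline's end it resets, or destroys itself if the character is invalid.
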(event `/Game/Blueprints/Interfaces/AttackInterface.AnimateAttack`
  (`self.SwingSword`))

(event `self.ReceiveTick`
  (params (DeltaSeconds :type "Float (single-precision)"))
  (set `self.Delta Seconds` DeltaSeconds))

(event `SwingSword`
  (`/Engine/EditorBlueprintResources/StandardMacros.DoOnce` false :!label _label
    (:`Completed`
      (`SceneComponent.ToggleVisibility` (`self.StaticMesh`) false)
      (bind _returnvalue (`KismetSystemLibrary.K2_SetTimerDelegate` (delegate `Timer`) 0.016 true))
      (set `self.TimerHandler` _returnvalue))))

(event `Timer`
  (bind _characterref (`self.CharacterRef`))
  (bind _staticmesh (`self.StaticMesh`))
  (bind _spline (`/Game/Blueprints/Character/BaseChracterBP.Spline` _characterref))
  (bind _duration (`SplineComponent.Duration` _spline))
  (bind _returnvalue (`KismetMathLibrary.Lerp` 0.0 _duration (`self.Time`)))
  (set `PrimitiveComponent.bGenerateOverlapEvents` true (`self.StaticMesh`))
  (`/Engine/EditorBlueprintResources/StandardMacros.IsValid` _characterref
    (:`Is Valid`
      (set `self.Time` (+ (* (`self.AttackSpeed`) (`self.Delta Seconds`)) (`self.Time`)))
      (`SceneComponent.K2_SetRelativeRotation` (`self.StaticMesh`) (struct :`Pitch` 90.0 :`Roll` 180.0) false false)
      (`self.K2_SetActorRelativeLocation` (.location (`SplineComponent.GetTransformAtTime` _spline _returnvalue "Local" false false)))
      (if (>= _returnvalue _duration)
        (`KismetSystemLibrary.K2_ClearAndInvalidateTimerHandle` (`self.TimerHandler`))
        (set `self.Time` 0.0)
        (`self.K2_SetActorRelativeLocation` (0.0 0.0 0.0))
        (set `PrimitiveComponent.bGenerateOverlapEvents` false _staticmesh)
        (`SceneComponent.ToggleVisibility` _staticmesh false)
        (goto _label :!via `Reset`)))
    (:`Is Not Valid`
      (`self.K2_DestroyActor`))))

(event `self.ReceiveBeginPlay`
  (bind _asbase_chracter_bp (cast `/Game/Blueprints/Character/BaseChracterBP` (`self.GetInstigator`)))
  (set `self.CharacterRef` _asbase_chracter_bp))

(event `self.StaticMesh.OnComponentBeginOverlap`
  (params (OverlappedComponent :type "PrimitiveComponent Object Reference") (OtherActor :type "Actor Object Reference") (OtherComp :type "PrimitiveComponent Object Reference") (OtherBodyIndex :type Integer) (bFromSweep :type Boolean) (SweepResult :type "HitResult Structure (by ref)"))
  (`self.Attack` OtherActor))

(fn `UserConstructionScript`)