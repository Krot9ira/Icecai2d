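; Base interactable actor that swings open once when the player interacts with it, like a lid or hatch.
; Interact calls Open, which plays a timeline that lerps the Scene component's relative rotation toward a fixed pitched angle and sets Opened.
; CheckInteractble reports it as interactable only while Opened is false.
; The lerp starts from the current rotation each update, so the motion eases rather than following the timeline linearly.
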(event `/Game/Blueprints/Interfaces/InteractionInterface.Interact`
  (params (Causer :type "Actor Object Reference"))
  (`self.Open`))

(event `Open`
  (bind (_direction _alpha) (`Timeline|OpenTimeline` :!via `PlayFromStart`)
    (:`Update`
      (`SceneComponent.K2_SetRelativeRotation` (`self.Scene`) (`KismetMathLibrary.RLerp` (`SceneComponent.RelativeRotation` (`self.Scene`)) (struct :`Roll` -80.0) _alpha true) false false)
      (set `self.Opened?` true))))

(event `self.ReceiveBeginPlay`)

(fn `CheckInteractble`
  (returns (`CanInteract?` :type Boolean))
  (return (not (`self.Opened?`))))

(fn `UserConstructionScript`)